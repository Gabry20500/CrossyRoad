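; BP_PG_BackDestroyer is a cleanup volume that destroys level pieces it overlaps, likely trailing play in a Crossy Road-style game.
; Its Move event shifts it by the given direction scaled by OffSet.
; On overlap, a long chain of exact class checks destroys terrain strips, scenery, planks, lily pads, vehicles and WoodDestroyer actors.
; Classes outside that hardcoded list are left untouched.
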(event `Move`
  (params (new_Direction :type Integer))
  (`self.K2_AddActorWorldOffset` (`KismetMathLibrary.MakeVector` (* new_Direction (`self.OffSet`)))))

(event `self.ReceiveActorBeginOverlap`
  (params (OtherActor :type "Actor Object Reference"))
  (bind _returnvalue (`GameplayStatics.GetObjectClass` OtherActor))
  (if (== _returnvalue "/Game/Terrain_Generation/Terrain_types/Inanimate/Trees/Tree.Tree_C")
    (`self.K2_DestroyActor` OtherActor :!label _label)
    (elif (== _returnvalue "/Game/Terrain_Generation/Terrain_types/Inanimate/Trees/TallTree.TallTree_C")
      (goto _label)
      (elif (== _returnvalue "/Game/Terrain_Generation/Terrain_types/Safe.Safe_C")
        (goto _label)
        (elif (== _returnvalue "/Game/Terrain_Generation/Terrain_types/Road.Road_C")
          (goto _label)
          (elif (== _returnvalue "/Game/Terrain_Generation/Terrain_types/River.River_C")
            (goto _label)
            (elif (== _returnvalue "/Game/Terrain_Generation/Terrain_types/Rail.Rail_C")
              (goto _label)
              (elif (== _returnvalue "/Game/Terrain_Generation/Terrain_types/Inanimate/WoodPlatform/WoodenPlate.WoodenPlate_C")
                (goto _label)
                (elif (== _returnvalue "/Game/Terrain_Generation/Terrain_types/Inanimate/WoodPlatform/LongPlate.LongPlate_C")
                  (goto _label)
                  (elif (== _returnvalue "/Game/Terrain_Generation/Terrain_types/Inanimate/WoodPlatform/LongLongPlate.LongLongPlate_C")
                    (goto _label)
                    (elif (== _returnvalue "/Game/Terrain_Generation/Terrain_types/WoodDestroyer.WoodDestroyer_C")
                      (goto _label)
                      (elif (== _returnvalue "/Game/Terrain_Generation/Terrain_types/Inanimate/WoodPlatform/Ninfee.Ninfee_C")
                        (goto _label)
                        (elif (== _returnvalue "/Game/Terrain_Generation/Terrain_types/Inanimate/Cars/BP_Ferrari.BP_Ferrari_C")
                          (goto _label)
                          (elif (== _returnvalue "/Game/Terrain_Generation/Terrain_types/Inanimate/Cars/BP_Camion.BP_Camion_C")
                            (goto _label)
                            (elif (== _returnvalue "/Game/Terrain_Generation/Terrain_types/Inanimate/Cars/BP_Camion_2.BP_Camion_2_C")
                              (goto _label)
                              (elif (== _returnvalue "/Game/Terrain_Generation/Terrain_types/Inanimate/Trees/Rock1.Rock1_C")
                                (goto _label)
                                (elif (== _returnvalue "/Game/Terrain_Generation/Terrain_types/Inanimate/Trees/Rock2.Rock2_C")
                                  (goto _label)
                                  (elif (== _returnvalue "/Game/Terrain_Generation/Terrain_types/Inanimate/Trees/Rock3.Rock3_C")
                                    (goto _label)
                                    (elif (== _returnvalue "/Game/Terrain_Generation/Terrain_types/Inanimate/Trees/Bush.Bush_C")
                                      (goto _label)
                                      (elif (== _returnvalue "/Game/Terrain_Generation/Terrain_types/Inanimate/Trees/BigTree.BigTree_C")
                                        (goto _label)
                                        (elif (== _returnvalue "/Game/Terrain_Generation/Terrain_types/Inanimate/Trees/BigTree2.BigTree2_C")
                                          (goto _label))))))))))))))))))))))

(fn `UserConstructionScript`)