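; BP_Camera is an auto-scrolling game camera that takes over the view at BeginPlay and advances along X.
; Each tick it moves at a base speed from DT_CameraSettings, switching to max speed when the player's projected screen Y passes a threshold.
; Scrolling stops once the player drops below the viewport.
; While the player stays within a central Y band, MoveComponentTo eases it toward a TargetXPos-based Y with fixed height and angle.
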(event `self.ReceiveBeginPlay`
  (bind _returnvalue (`GameplayStatics.GetActorOfClass` "/Game/BluePrint/BP_Player.BP_Player_C"))
  (set `self.Player` _returnvalue)
  (bind _returnvalue_2 (`GameplayStatics.GetActorOfClass` "BP_Camera_C"))
  (`PlayerController.SetViewTargetWithBlend` (`GameplayStatics.GetPlayerController` 0) _returnvalue_2 0.0 "VTBlend_Linear" 0.0 false)
  (bind _returnvalue_3 (`|GetDataTableRow` "/Game/BluePrint/Data_Table/DT_CameraSettings.DT_CameraSettings" "First")
    (:`then`
      (set `self.Camera Settings` _returnvalue_3))))

(event `self.ReceiveTick`
  (params (DeltaSeconds :type "Float (single-precision)"))
  (bind (_returnvalue_x _returnvalue_y) (`KismetMathLibrary.BreakVector2D` (`WidgetLayoutLibrary.GetViewportSize`)))
  (bind _defaultsceneroot (`self.DefaultSceneRoot`))
  (bind _returnvalue_x_2 (`KismetMathLibrary.BreakVector` (`SceneComponent.K2_GetComponentLocation` _defaultsceneroot)))
  (bind _screenposition (`GameplayStatics.ProjectWorldToScreen` (`GameplayStatics.GetPlayerController` 0) (`self.K2_GetActorLocation` (`GameplayStatics.GetPlayerCharacter` 0))))
  (bind (_returnvalue_x_3 _returnvalue_y_2) (`KismetMathLibrary.BreakVector` (`SceneComponent.K2_GetComponentLocation` (`Character.CapsuleComponent` (`self.Player`)))))
  (`|ExecutionSequence`
    (:`then_0`
      (bind _output_get (set `self.RepositionCamera` (< (`.Y` (`KismetMathLibrary.BreakVector2D` _screenposition)) (- (/ _returnvalue_y (`.ScreenYTreshold_14_FBC716FF43B317CC5058C4A75CC0335A` (break `/Game/BluePrint/Data_Table/ST_CameraSettings` (`self.Camera Settings`)))) _returnvalue_y))))
      (if (> (`.Y` (`KismetMathLibrary.BreakVector2D` _screenposition)) _returnvalue_y)
        _
        (elif _output_get
          (`SceneComponent.K2_AddRelativeLocation` (`self.DefaultSceneRoot`) (`KismetMathLibrary.MakeVector` (`.MaxSpeed_13_ECE473CC4EF62A0018D855BC09E994CA` (break `/Game/BluePrint/Data_Table/ST_CameraSettings` (`self.Camera Settings`)))) true false)
          (else
            (`SceneComponent.K2_AddRelativeLocation` (`self.DefaultSceneRoot`) (`KismetMathLibrary.MakeVector` (`.BaseSpeed_9_2C08460E4CA951D354D4B4A826FD84C9` (break `/Game/BluePrint/Data_Table/ST_CameraSettings` (`self.Camera Settings`)))) false true)))))
    (:`then_1`
      (if (not (or (< _returnvalue_y_2 -200.0) (> _returnvalue_y_2 200.0)))
        (`KismetSystemLibrary.MoveComponentTo` _defaultsceneroot (`KismetMathLibrary.MakeVector` _returnvalue_x_2 (+ (`self.Target X pos`) 130.0) 307.649658) (struct :`Pitch` -52.21286 :`Yaw` -28.963623 :`Roll` 11.524208))))))

(fn `UserConstructionScript`)