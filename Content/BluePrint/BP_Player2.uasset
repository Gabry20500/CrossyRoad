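; Player character for a Crossy Road-style game, hopping a chicken across lanes with cars, trains and rivers.
; Axis input launches timed hops and turns the mesh via timelines; a cooldown gates movement.
; Forward and backward hops update the line count and shift a spawned BackDestroyer, with forward progress raising score and triggering Spawn_Manager generation.
; Vehicle hits squash the chicken and drowning hides it, both showing GameOver; Escape toggles pause.
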(event `self.ReceiveBeginPlay`
  (bind (_returnvalue_x _returnvalue_y _returnvalue_z) (`KismetMathLibrary.BreakVector` (`SceneComponent.K2_GetComponentLocation` (`self.CapsuleComponent`))))
  ;[1 1 1] Initializing Obj references
  (bind _returnvalue (`|SpawnActorFromClass` "/Game/Blueprint/BP_PG_BackDestroyer.BP_PG_BackDestroyer_C" (`KismetMathLibrary.MakeTransform` (`KismetMathLibrary.MakeVector` (- _returnvalue_x 1000.0) _returnvalue_y _returnvalue_z)) "Undefined" "OverrideRootScale" null null))
  (set `self.BackDestroyer` _returnvalue)
  (bind _returnvalue_2 (`GameplayStatics.GetActorOfClass` "/Game/Terrain_Generation/Spawn_Manager.Spawn_Manager_C"))
  (set `self.SpawnManager` _returnvalue_2))

(event `InputAxis|Foreward`
  (params (AxisValue :type "Float (single-precision)"))
  (bind _returnvalue (* AxisValue 230.0))
  (bind _recordlinereached (`self.RecordLineReached`))
  (bind _score (`self.Score`))
  (bind _recordlinereached_2 (`self.RecordLineReached`))
  (bind _chicken (`self.Chicken`))
  (bind _chicken_2 (`self.Chicken`))
  ;[1 1 1] Movement
  (if (and (> (`KismetMathLibrary.Abs` AxisValue) 0.3) (`self.CanMove`))
    (`self.MovementCooldown`)
    (`self.LaunchCharacter` (`KismetMathLibrary.MakeVector` _returnvalue 0.0 200.0) true true)
    (if (> _returnvalue 0.1)
      (set `self.RecordLineReached` (+ (`self.RecordLineReached`) 1))
      (`|ExecutionSequence`
        (:`then_0`
          (if (> _recordlinereached _score)
            (set `self.Score` _recordlinereached)
            (else
              (set `self.Score` _score))))
        (:`then_1`
          (`/Game/Blueprint/BP_PG_BackDestroyer.Move` (`self.BackDestroyer`) 1)
          (if (>= _recordlinereached_2 (+ (`self.LastCheckedLine`) (`self.DelayLineNum`)))
            (bind _output_get (set `self.LastCheckedLine` _recordlinereached_2))
            (`/Game/Terrain_Generation/Spawn_Manager.Generate` (`self.SpawnManager`) _output_get))
          ;[1 1 1] Rotation in Foreward Movement
          (if (> AxisValue 0.3) :!label _label
            (bind (_direction _newtrack_0) (`Timeline|Rotation` :!via `PlayFromStart`)
              (:`Update`
                (`SceneComponent.K2_SetWorldRotation` _chicken (`KismetMathLibrary.RLerp` (`SceneComponent.K2_GetComponentRotation` _chicken) (struct :`Yaw` -180.0) _newtrack_0 true) false false)))
            (else
              (bind (_direction_2 _newtrack_0_2) (`Timeline|Timeline_0` :!via `PlayFromStart`)
                (:`Update`
                  (`SceneComponent.K2_SetWorldRotation` _chicken_2 (`KismetMathLibrary.RLerp` (`SceneComponent.K2_GetComponentRotation` _chicken_2) (struct) _newtrack_0_2 true) false false)))))))
      (else
        (set `self.RecordLineReached` (- (`self.RecordLineReached`) 1))
        (`/Game/Blueprint/BP_PG_BackDestroyer.Move` (`self.BackDestroyer`) -1)
        (goto _label)))))

(event `InputAxis|Side `
  (params (AxisValue :type "Float (single-precision)"))
  (bind _chicken (`self.Chicken`))
  (bind _chicken_2 (`self.Chicken`))
  ;[1 1 1] Movement
  (if (and (> (`KismetMathLibrary.Abs` AxisValue) 0.3) (`self.CanMove`))
    (`self.MovementCooldown`)
    (`self.LaunchCharacter` (`KismetMathLibrary.MakeVector` 0.0 (* AxisValue 230.0) 200.0) true true)
    ;[1 1 1] Rotation in Side Movement
    (if (> AxisValue 0.3)
      (bind (_direction _newtrack_0) (`Timeline|Timeline_1` :!via `PlayFromStart`)
        (:`Update`
          (`SceneComponent.K2_SetWorldRotation` _chicken_2 (`KismetMathLibrary.RLerp` (`SceneComponent.K2_GetComponentRotation` _chicken_2) (struct :`Yaw` -90.0) _newtrack_0 true) false false)))
      (else
        (bind (_direction_2 _newtrack_0_2) (`Timeline|Timeline_2` :!via `PlayFromStart`)
          (:`Update`
            (`SceneComponent.K2_SetWorldRotation` _chicken (`KismetMathLibrary.RLerp` (`SceneComponent.K2_GetComponentRotation` _chicken) (struct :`Yaw` 90.0) _newtrack_0_2 true) false false)))))))

(event `MovementCooldown`
  ;[1 1 1] Create delay for movement
  (`/Engine/EditorBlueprintResources/StandardMacros.DoOnce` false :!label _label_2
    (:`Completed`
      (set `self.CanMove` false)
      (`KismetSystemLibrary.Delay` 0.5)
      (set `self.CanMove` true)
      (goto _label_2 :!via `Reset`))))

(event `Key|Escape`
  (params (Key :type "Key Structure"))
  ;[1 1 1] Pause Menu
  (:`Pressed`
    (`/Engine/EditorBlueprintResources/StandardMacros.FlipFlop`
      (:`A`
        (bind _returnvalue (`|CreateWidget` "/Game/Blueprint/HUD/WB_PlayGame.WB_PlayGame_C"))
        (`UserWidget.AddToViewport` _returnvalue 0)
        (`GameplayStatics.SetGamePaused` true)
        (set `PlayerController.bShowMouseCursor` true (`GameplayStatics.GetPlayerController` 0)))
      (:`B`
        (`Widget.RemoveFromParent` _returnvalue)
        (`GameplayStatics.SetGamePaused` false)
        (set `PlayerController.bShowMouseCursor` false (`GameplayStatics.GetPlayerController` 0))))))

(event `self.Box.OnComponentBeginOverlap`
  (params (OverlappedComponent :type "PrimitiveComponent Object Reference") (OtherActor :type "Actor Object Reference") (OtherComp :type "PrimitiveComponent Object Reference") (OtherBodyIndex :type Integer) (bFromSweep :type Boolean) (SweepResult :type "HitResult Structure (by ref)"))
  (bind _returnvalue (`GameplayStatics.GetObjectClass` OtherActor))
  ;[1 1 1] Hit By Something
  (if (== _returnvalue "/Game/Terrain_Generation/Terrain_types/Inanimate/Cars/BP_Blue_Car.BP_Blue_Car_C")
    (`/Engine/EditorBlueprintResources/StandardMacros.DoOnce` false :!label _label_3
      (:`Completed`
        (`self.Player Overlapped`)))
    (elif (== _returnvalue "/Game/Terrain_Generation/Terrain_types/Inanimate/Cars/BP_Red_Car.BP_Red_Car_C")
      (goto _label_3)
      (elif (== _returnvalue "/Game/Terrain_Generation/Terrain_types/Inanimate/BP_Train.BP_Train_C")
        (goto _label_3)))))

(event `Drown In River`
  ;[1 1 1] Drown in river
  (`SceneComponent.SetWorldScale3D` (`self.Chicken`) (0.0 0.0 0.0))
  (bind _returnvalue (`|CreateWidget` "/Game/GUI/GameOver.GameOver_C"))
  (`UserWidget.AddToViewport` _returnvalue 0)
  (set `PlayerController.bShowMouseCursor` true (`GameplayStatics.GetPlayerController` 0))
  (`self.DisableInput` (`GameplayStatics.GetPlayerController` 0)))

(fn `Player Overlapped`
  ;[1 1 1] Hitted By Car
  (`SceneComponent.SetWorldScale3D` (`self.Chicken`) (1.0 1.0 0.1))
  (bind _returnvalue (`|CreateWidget` "/Game/GUI/GameOver.GameOver_C"))
  (`UserWidget.AddToViewport` _returnvalue 0)
  (set `PlayerController.bShowMouseCursor` true (`GameplayStatics.GetPlayerController` 0))
  (`self.DisableInput` (`GameplayStatics.GetPlayerController` 0)))

(fn `UserConstructionScript`)