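; BP_Player is the hopping chicken character for what appears to be a Crossy Road-style game with cars and a river.
; Forward and side axis input launches it in short hops while timelines turn the mesh toward the move direction.
; A DoOnce and half-second delay on CanMove space out the hops.
; HitByCar flattens the chicken and DrownInRiver hides it by scale; both show GameOver and the cursor and zero walk speed.
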(event `InputAxis|MoveForeward`
  (params (AxisValue :type "Float (single-precision)"))
  (bind _chicken (`self.Chicken`))
  (bind _chicken_2 (`self.Chicken`))
  ;[1 1 1] Movement
  (if (and (> (`KismetMathLibrary.Abs` AxisValue) 0.3) (`self.CanMove`))
    (`self.MovementCooldown`)
    (`self.LaunchCharacter` (`KismetMathLibrary.MakeVector` (* AxisValue 235.220688) 0.0 200.0) true true)
    ;[1 1 1] Rotation in Foreward Movement
    (if (> AxisValue 0.3)
      (bind (_direction _newtrack_0) (`Timeline|Rotation` :!via `PlayFromStart`)
        (:`Update`
          (`SceneComponent.K2_SetWorldRotation` _chicken (`KismetMathLibrary.RLerp` (`SceneComponent.K2_GetComponentRotation` _chicken) (struct :`Yaw` -90.0) _newtrack_0 true) false false)))
      (else
        (bind (_direction_2 _newtrack_0_2) (`Timeline|Timeline_0` :!via `PlayFromStart`)
          (:`Update`
            (`SceneComponent.K2_SetWorldRotation` _chicken_2 (`KismetMathLibrary.RLerp` (`SceneComponent.K2_GetComponentRotation` _chicken_2) (struct :`Yaw` 90.0) _newtrack_0_2 true) false false)))))))

(event `InputAxis|Side Movement`
  (params (AxisValue :type "Float (single-precision)"))
  (bind _chicken (`self.Chicken`))
  (bind _chicken_2 (`self.Chicken`))
  ;[1 1 1] Movement
  (if (and (> (`KismetMathLibrary.Abs` AxisValue) 0.3) (`self.CanMove`))
    (`self.MovementCooldown`)
    (`self.LaunchCharacter` (`KismetMathLibrary.MakeVector` 0.0 (* AxisValue 250.0) 200.0) true true)
    ;[1 1 1] Rotation in Side Movement
    (if (> AxisValue 0.3)
      (bind (_direction _newtrack_0) (`Timeline|Timeline_1` :!via `PlayFromStart`)
        (:`Update`
          (`SceneComponent.K2_SetWorldRotation` _chicken_2 (`KismetMathLibrary.RLerp` (`SceneComponent.K2_GetComponentRotation` _chicken_2) (struct) _newtrack_0 true) false false)))
      (else
        (bind (_direction_2 _newtrack_0_2) (`Timeline|Timeline_2` :!via `PlayFromStart`)
          (:`Update`
            (`SceneComponent.K2_SetWorldRotation` _chicken (`KismetMathLibrary.RLerp` (`SceneComponent.K2_GetComponentRotation` _chicken) (struct :`Yaw` -180.0) _newtrack_0_2 true) false false)))))))

(event `MovementCooldown`
  ;[1 1 1] Create delay for movement
  (`/Engine/EditorBlueprintResources/StandardMacros.DoOnce` false :!label _label
    (:`Completed`
      (set `self.CanMove` false)
      (`KismetSystemLibrary.Delay` 0.5)
      (set `self.CanMove` true)
      (goto _label :!via `Reset`))))

(event `Hit By Car`
  ;[1 1 1] Hitted By Car
  (`SceneComponent.SetWorldScale3D` (`self.Chicken`) (1.0 1.0 0.1))
  (bind _returnvalue (`|CreateWidget` "/Game/GUI/GameOver.GameOver_C"))
  (`UserWidget.AddToViewport` _returnvalue 0)
  (set `PlayerController.bShowMouseCursor` true (`GameplayStatics.GetPlayerController` 0))
  (set `CharacterMovementComponent.MaxWalkSpeed` 0.0 (`self.CharacterMovement`)))

(event `Drown In River`
  ;[1 1 1] Drown in river
  (`SceneComponent.SetWorldScale3D` (`self.Chicken`) (0.0 0.0 0.0))
  (bind _returnvalue (`|CreateWidget` "/Game/GUI/GameOver.GameOver_C"))
  (`UserWidget.AddToViewport` _returnvalue 0)
  (set `PlayerController.bShowMouseCursor` true (`GameplayStatics.GetPlayerController` 0))
  (set `CharacterMovementComponent.MaxWalkSpeed` 0.0 (`self.CharacterMovement`)))

(fn `UserConstructionScript`)