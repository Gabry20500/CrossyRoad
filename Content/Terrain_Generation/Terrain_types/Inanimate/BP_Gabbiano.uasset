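; BP_Gabbiano is an inanimate terrain actor, named as a seagull, that makes swooping moves toward the player.
; BeginPlay caches BP_Player and the mesh's starting world transform, and prints a debug label.
; Tick drives a short MoveComponentTo of the root toward the player capsule's relative location with a 180-degree rotation, then calls Return to move it back to the stored position and zero rotation.
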(event `self.ReceiveBeginPlay`
  (`KismetSystemLibrary.PrintString` "GABBIANO")
  (bind _returnvalue (`GameplayStatics.GetActorOfClass` "/Game/BluePrint/BP_Player.BP_Player_C"))
  (set `self.PG` _returnvalue)
  (set `self.InitialPosition` (`SceneComponent.K2_GetComponentToWorld` (`self.Mesh`))))

(event `self.ReceiveTick`
  (params (DeltaSeconds :type "Float (single-precision)"))
  (`KismetSystemLibrary.MoveComponentTo` (`self.DefaultSceneRoot`) (`SceneComponent.RelativeLocation` (`Character.CapsuleComponent` (`self.PG`))) (struct :`Yaw` 180.0) false false 0.2 true)
  (`self.Return`))

(event `Return`
  (bind _initialposition_location (`KismetMathLibrary.BreakTransform` (`self.InitialPosition`)))
  (`KismetSystemLibrary.MoveComponentTo` (`self.DefaultSceneRoot`) _initialposition_location (struct) false false 0.2 true))

(fn `UserConstructionScript`)