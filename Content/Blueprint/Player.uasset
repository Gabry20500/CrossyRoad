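; Player Blueprint that moves in fixed, grid-like steps from four directional input actions.
; Each press calls TryMove, which offsets TargetPos and clears CanMove until a short timer calls EnableCanMove, limiting the step rate.
; Tick continuously issues MoveComponentTo on DefaultSceneRoot toward TargetPos, so each step glides instead of snapping.
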(event `InputAction|Move_Forward`
  (params (Key :type "Key Structure"))
  (:`Pressed`
    (`self.TryMove` (100.0 0.0 0.0))))

(event `self.ReceiveTick`
  (params (DeltaSeconds :type "Float (single-precision)"))
  (`KismetSystemLibrary.MoveComponentTo` (`self.DefaultSceneRoot`) (`self.TargetPos`) (struct) false false 0.1))

(event `InputAction|Move_Left`
  (params (Key :type "Key Structure"))
  (:`Pressed`
    (`self.TryMove` (0.0 -100.0 0.0))))

(event `InputAction|Move_Right`
  (params (Key :type "Key Structure"))
  (:`Pressed`
    (`self.TryMove` (0.0 100.0 0.0))))

(event `InputAction|Move_Backward`
  (params (Key :type "Key Structure"))
  (:`Pressed`
    (`self.TryMove` (-100.0 0.0 0.0))))

(fn `EnableCanMove`
  (set `self.CanMove?` true))

(fn `TryMove`
  (params (Direction :type "Vector Structure"))
  (if (`self.CanMove?`)
    (set `self.TargetPos` (+ Direction (`self.TargetPos`)))
    (set `self.CanMove?` false)
    (`KismetSystemLibrary.K2_SetTimer` null "EnableCanMove" 0.3)))

(fn `UserConstructionScript`)